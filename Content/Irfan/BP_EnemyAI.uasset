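; Enemy AI character, apparently a zombie, that chases the player on sight and attacks in melee.
; PawnSensing starts AIMoveTo; on success it plays a montage and damages Player-tagged actors in a sphere overlap at an arrow component.
; CanAttack gates attacks for the montage length, while Tick halts movement and turns a widget toward the camera.
; Damage reduces health; a hit received at zero or below destroys it.
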(event OnSeePawn(PawnSensing)
  (params (Pawn :type Pawn%20Object%20Reference))
  (Variables|Default|SetisSeeingPlayer? true)
  (CallFunction|FollowPlayer))

(event Custom|FollowPlayer
  (if (Variables|Default|GetisSeeingPlayer?)
    (AI|AIMoveTo self "0, 0, 0" (Game|GetPlayerCharacter 0) 7e+01 false
      (:OnSuccess
        (if (Variables|Default|GetcanAttack?)
          (Variables|Default|SetcanAttack? false)
          (Development|PrintString "enemy attack")
          (bind _returnvalue (Animation|PlayAnimMontage "/Game/Characters/Zombie_Attack_Montage.Zombie_Attack_Montage" 1.0 "None"))
          (bind _outactors (Collision|SphereOverlapActors (Transformation|GetWorldLocation (Variables|Default|GetArrow1)) 1e+02 (Variables|Default|GetObject%20Types) 0))
          (bind _array_element (Utilities|Array|ForEachLoopwithBreak _outactors)
            (:LoopBody
              (if (Actor|ActorHasTag _array_element "Player")
                (Game|Damage|ApplyDamage _array_element 5.0 0 0)))
            (:Completed
              (Utilities|FlowControl|Delay _returnvalue)
              (Variables|Default|SetcanAttack? true))))))
    (else
      (Variables|Default|SetisSeeingPlayer? false))))

(event EventBeginPlay)

(event Collision|EventActorBeginOverlap
  (params (OtherActor :type Actor%20Object%20Reference)))

(event EventTick
  (params (DeltaSeconds :type Float%20%28single-precision%29))
  (Utilities|FlowControl|Sequence
    (:then_0
      (if (not (Variables|Default|GetcanAttack?))
        (Components|Movement|StopMovementImmediately (Variables|Character|GetCharacterMovement))))
    (:then_1
      (Transformation|SetWorldRotation (Variables|Default|GetWidget) (Math|Rotator|FindLookatRotation (Transformation|GetWorldLocation (Variables|Default|GetWidget)) (Transformation|GetWorldLocation (Variables|/Script/Engine.PlayerCameraManager|GetTransformComponent (Game|GetPlayerCameraManager 0)))) false false))))

(event Game|Damage|EventAnyDamage
  (params (Damage :type Float%20%28single-precision%29) (DamageType :type Damage%20Type%20Object%20Reference) (InstigatedBy :type Controller%20Object%20Reference) (DamageCauser :type Actor%20Object%20Reference))
  (if (> (Variables|Default|GetHeath) 0.0)
    (Variables|Default|SetHeath (- (Variables|Default|GetHeath) Damage))
    (Development|PrintString "Damage recived")
    (else
      (Actor|DestroyActor))))

(fn ConstructionScript)